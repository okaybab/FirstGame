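; Actor that moves a Cube back and forth along its Spline in a ping-pong loop.
; Tick plays or reverses a Timeline based on IsFoward, and the Timeline flips that flag when finished.
; Each update maps the Timeline value to spline length and applies the local location and rotation to the Cube, keeping its scale.
; MoveFoward and MoveBackward offer distance-stepped movement but are not called in these graphs.
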(event `self.ReceiveTick`
  (params (DeltaSeconds :type "Float (single-precision)"))
  (bind _spline (`self.Spline`))
  (bind _cube (`self.Cube`))
  (if (`self.IsFoward`)
    (bind (_direction _value) (`Timeline|타임라인_0` :!label _label)
      (:`Update`
        (bind (_returnvalue_location _returnvalue_rotation) (`KismetMathLibrary.BreakTransform` (`SplineComponent.GetTransformAtDistanceAlongSpline` _spline (* _value (`SplineComponent.GetSplineLength` _spline)) "Local" false)))
        (`SceneComponent.K2_SetRelativeTransform` _cube (`KismetMathLibrary.MakeTransform` _returnvalue_location _returnvalue_rotation (`SceneComponent.RelativeScale3D` _cube)) false false))
      (:`Finished`
        (set `self.IsFoward` (not (`self.IsFoward`)))))
    (else
      (goto _label :!via `Reverse`))))

(fn `Move Foward`
  (params (Distance :type "Float (double-precision)"))
  (bind _spline (`self.Spline`))
  (bind _cube (`self.Cube`))
  (bind _output_get (set `self.Distance` (+ (`self.Distance`) Distance)))
  (`SceneComponent.K2_SetRelativeTransform` _cube (`KismetMathLibrary.MakeTransform` (`SplineComponent.GetLocationAtDistanceAlongSpline` _spline _output_get "Local") (`SplineComponent.GetRotationAtDistanceAlongSpline` _spline _output_get "Local") (`SceneComponent.RelativeScale3D` _cube)) false false)
  (if (> (`self.Distance`) (`SplineComponent.GetSplineLength` (`self.Spline`)))
    (set `self.IsFoward` false)))

(fn `MoveBackward`
  (params (B :type "Float (double-precision)"))
  (bind _spline (`self.Spline`))
  (bind _cube (`self.Cube`))
  (bind _output_get (set `self.Distance` (- (`self.Distance`) B)))
  (`SceneComponent.K2_SetRelativeTransform` _cube (`KismetMathLibrary.MakeTransform` (`SplineComponent.GetLocationAtDistanceAlongSpline` _spline _output_get "Local") (`SplineComponent.GetRotationAtDistanceAlongSpline` _spline 0.0 "Local") (`SceneComponent.RelativeScale3D` _cube)) false false)
  (if (<= (`self.Distance`) 0.0)
    (set `self.IsFoward` true)))

(fn `UserConstructionScript`)