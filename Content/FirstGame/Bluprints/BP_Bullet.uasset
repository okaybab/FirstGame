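; BP_Bullet is a homing projectile that, on BeginPlay, targets the player pawn.
; A looping timer runs MoveRotationTarget, gradually turning the sphere toward the target while moving it forward; MoveBullet and MoveUFO are unused variants.
; Overlapping a BP_FirstGamePerson triggers its ragdoll, enables sphere physics and destroys the bullet after a delay.
; The hit clears only the MoveBullet timer, so the active homing timer continues until destruction.
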(event `self.ReceiveBeginPlay`
  (`self.OnShoot` (`GameplayStatics.GetPlayerPawn` 0)))

(event `self.Sphere.OnComponentBeginOverlap`
  (params (OverlappedComponent :type "PrimitiveComponent Object Reference") (OtherActor :type "Actor Object Reference") (OtherComp :type "PrimitiveComponent Object Reference") (OtherBodyIndex :type Integer) (bFromSweep :type Boolean) (SweepResult :type "HitResult Structure (by ref)"))
  (bind _asbp_first_game_person (cast `/Game/FirstGame/Gamemode/BP_FirstGamePerson` OtherActor))
  (`/Game/FirstGame/Gamemode/BP_FirstGamePerson.DoRacdoll` _asbp_first_game_person)
  (`KismetSystemLibrary.K2_ClearTimer` null "MoveBullet")
  (`PrimitiveComponent.SetSimulatePhysics` (`self.Sphere`) true)
  (`KismetSystemLibrary.Delay` 3.0)
  (`self.K2_DestroyActor`))

(fn `Move Rotation Target`
  (bind _sphere (`self.Sphere`))
  (bind _sphere_2 (`self.Sphere`))
  (`/Engine/EditorBlueprintResources/StandardMacros.IsValid` (`self.Target`)
    (:`Is Valid`
      ;[1 1 1] Lerp
      (`SceneComponent.K2_SetWorldRotation` _sphere_2 (`KismetMathLibrary.RLerp` (`SceneComponent.K2_GetComponentRotation` _sphere_2) (`KismetMathLibrary.FindLookAtRotation` (`SceneComponent.K2_GetComponentLocation` (`self.Sphere`)) (`self.K2_GetActorLocation` (`self.Target`))) 0.01 true) false false)
      ;[1 1 1] bullet 속도
      (`SceneComponent.K2_AddWorldOffset` _sphere (* (`SceneComponent.GetForwardVector` _sphere) (* 0.01 (`self.speed`))) false false))))

(fn `MoveBullet`
  (bind _sphere (`self.Sphere`))
  (`/Engine/EditorBlueprintResources/StandardMacros.IsValid` (`self.Target`)
    (:`Is Valid`
      ;[1 1 1] bullet 속도
      (`SceneComponent.K2_AddWorldOffset` _sphere (* (`SceneComponent.GetForwardVector` _sphere) (* 0.01 (`self.speed`))) false false))))

(fn `MoveUFO`
  (bind _returnvalue (* 0.01 (`self.speed`)))
  (`/Engine/EditorBlueprintResources/StandardMacros.IsValid` (`self.Target`)
    (:`Is Valid`
      (`SceneComponent.K2_AddWorldOffset` (`self.Sphere`) (* (`KismetMathLibrary.GetForwardVector` (`KismetMathLibrary.FindLookAtRotation` (`SceneComponent.K2_GetComponentLocation` (`self.Sphere`)) (`self.K2_GetActorLocation` (`self.Target`)))) _returnvalue) false false)
      (`KismetSystemLibrary.PrintString` (`KismetStringLibrary.Conv_DoubleToString` _returnvalue)))))

(fn `OnShoot`
  (params (Target :type "Actor Object Reference"))
  (bind _sphere (`self.Sphere`))
  (set `self.Target` Target)
  (`SceneComponent.K2_SetWorldRotation` _sphere (`KismetMathLibrary.FindLookAtRotation` (`SceneComponent.K2_GetComponentLocation` _sphere) (`self.K2_GetActorLocation` (`self.Target`))) false false)
  (`KismetSystemLibrary.K2_SetTimer` null "MoveRotationTarget" 0.01 true))

(fn `UserConstructionScript`)