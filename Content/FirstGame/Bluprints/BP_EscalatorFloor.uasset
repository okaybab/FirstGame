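; BP_EscalatorFloor is a moving escalator step that travels repeatedly along a spline.
; A looping 0.01-second timer advances its distance by Speed and snaps the actor's transform to that point, without sweeping.
; Past the spline's end, it hides the cube and disables collision, stops the timer, then after a short delay returns to the start, restores both and restarts movement.
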(event `self.ReceiveBeginPlay`
  (`KismetSystemLibrary.K2_SetTimer` null "UpdateMoveFloor" 0.01 true))

(event `self.ReceiveTick`
  (params (DeltaSeconds :type "Float (single-precision)")))

(fn `SetStartPoint`
  (bind _cube (`self.Cube`))
  (set `self.distance` 0.0)
  (`self.K2_SetActorTransform` (`SplineComponent.GetTransformAtDistanceAlongSpline` (`self.spline`) 0.0 "World" false))
  (`SceneComponent.SetVisibility` _cube true false)
  (`PrimitiveComponent.SetCollisionEnabled` _cube "QueryAndPhysics")
  (`KismetSystemLibrary.K2_SetTimer` null "UpdateMoveFloor" 0.01 true))

(fn `UpdateMoveFloor`
  (bind _cube (`self.Cube`))
  (bind _output_get (set `self.distance` (+ (* 0.01 (`self.speed`)) (`self.distance`))))
  (`self.K2_SetActorTransform` (`SplineComponent.GetTransformAtDistanceAlongSpline` (`self.spline`) _output_get "World" false))
  (if (> (`self.distance`) (`SplineComponent.GetSplineLength` (`self.spline`)))
    (`SceneComponent.SetVisibility` _cube false false)
    (`PrimitiveComponent.SetCollisionEnabled` _cube "NoCollision")
    (`KismetSystemLibrary.K2_SetTimer` null "SetStartPoint" 0.1)
    (`KismetSystemLibrary.K2_ClearTimer` null "UpdateMoveFloor")))

(fn `UserConstructionScript`)