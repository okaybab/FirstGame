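; BP_Weapon is a weapon pickup actor that can be attached to a character and dropped back into the world.
; When BP_FirstGamePerson overlaps its pickup collision, it passes its location to BP_MyHUD_Child to update the pickup position.
; AttachWeapon disables mesh physics and collision, then snaps the static mesh component, not the actor, to a character socket.
; DettachWeapon restores both and detaches the mesh in place.
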(event `self.ReceiveTick`
  (params (DeltaSeconds :type "Float (single-precision)")))

(event `self.PickupColision.OnComponentBeginOverlap`
  (params (OverlappedComponent :type "PrimitiveComponent Object Reference") (OtherActor :type "Actor Object Reference") (OtherComp :type "PrimitiveComponent Object Reference") (OtherBodyIndex :type Integer) (bFromSweep :type Boolean) (SweepResult :type "HitResult Structure (by ref)"))
  (cast `/Game/FirstGame/Gamemode/BP_FirstGamePerson` OtherActor)
  (bind _asbp_my_hud_child (cast `/Game/FirstGame/Gamemode/BP_MyHUD_Child` (`PlayerController.GetHUD` (`GameplayStatics.GetPlayerController` 0))))
  (`/Game/FirstGame/Gamemode/BP_MyHUD_Child.Update Pick Up Posision` _asbp_my_hud_child (`self.K2_GetActorLocation`)))

(fn `AttachWeapon`
  (params (Character :type "Character Object Reference"))
  (returns (result :type Boolean))
  (bind _staticmesh (`self.StaticMesh`))
  (`PrimitiveComponent.SetSimulatePhysics` _staticmesh false)
  (`PrimitiveComponent.SetCollisionEnabled` _staticmesh "NoCollision")
  (bind _returnvalue (`SceneComponent.K2_AttachToComponent` _staticmesh (`Character.Mesh` Character) (`self.Socket Name`) "SnapToTarget" "SnapToTarget" "KeepWorld" true))
  (return _returnvalue))

(fn `DettachWeapon`
  (params (Character :type "Character Object Reference"))
  (returns (result :type Boolean))
  (bind _staticmesh (`self.StaticMesh`))
  (`PrimitiveComponent.SetCollisionEnabled` _staticmesh "QueryAndPhysics")
  (`PrimitiveComponent.SetSimulatePhysics` _staticmesh true)
  (`SceneComponent.K2_DetachFromComponent` _staticmesh "KeepWorld" "KeepWorld" "KeepWorld" true)
  (return true))

(fn `UserConstructionScript`)