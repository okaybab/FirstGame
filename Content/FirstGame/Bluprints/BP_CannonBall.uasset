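; Cannon actor that tracks the player pawn and fires a physics ball every two seconds.
; Tick smoothly turns the Arrow toward the player with a rotator lerp, serving as muzzle and aim.
; Do Shoot reuses one Ball, snapping it to the Arrow, clearing velocity and applying a forward impulse.
; Hitting a BP_SwatPerson triggers ragdoll, an outward impulse, explosion sound and particles; a BP_FirstGamePerson ragdoll branch is unwired.
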(event `self.ReceiveBeginPlay`
  (set `self.Target` (`GameplayStatics.GetPlayerPawn` 0))
  (`self.Do Shoot`)
  (`KismetSystemLibrary.K2_SetTimer` null "Do Shoot" 2.0 true))

(event `self.ReceiveTick`
  (params (DeltaSeconds :type "Float (single-precision)"))
  (bind _arrow (`self.Arrow`))
  (`SceneComponent.K2_SetWorldRotation` _arrow (`KismetMathLibrary.RLerp` (`SceneComponent.K2_GetComponentRotation` _arrow) (`KismetMathLibrary.FindLookAtRotation` (`SceneComponent.K2_GetComponentLocation` _arrow) (`self.K2_GetActorLocation` (`self.Target`))) 0.05 true) false false))

(event `self.Ball.OnComponentHit`
  (params (HitComponent :type "PrimitiveComponent Object Reference") (OtherActor :type "Actor Object Reference") (OtherComp :type "PrimitiveComponent Object Reference") (NormalImpulse :type "Vector Structure") (Hit :type "HitResult Structure (by ref)"))
  (`KismetSystemLibrary.PrintString` (`KismetSystemLibrary.GetDisplayName` OtherActor))
  (bind _asbp_swat_person (cast `/Game/FirstGame/Gamemode/BP_SwatPerson` OtherActor))
  (`/Game/FirstGame/Gamemode/BP_SwatPerson.DoRacdoll` _asbp_swat_person)
  (bind _mesh (`Character.Mesh` _asbp_swat_person))
  (`PrimitiveComponent.AddImpulse` _mesh (* (`KismetMathLibrary.GetForwardVector` (`KismetMathLibrary.FindLookAtRotation` (`SceneComponent.K2_GetComponentLocation` (`self.Ball`)) (`self.K2_GetActorLocation` _asbp_swat_person))) 100000.0) "None" false)
  (`AudioComponent.Play` (`self.Explosion_Cue`) 0.0)
  (`GameplayStatics.SpawnEmitterAtLocation` "/Game/StarterContent/Particles/P_Explosion.P_Explosion" (`SceneComponent.K2_GetComponentLocation` _mesh) (struct) (3.0 3.0 3.0)))

(fn `Do Shoot`
  (bind _ball (`self.Ball`))
  (bind _arrow (`self.Arrow`))
  (`SceneComponent.K2_SetWorldLocationAndRotation` (`self.Ball`) (`SceneComponent.K2_GetComponentLocation` _arrow) (`SceneComponent.K2_GetComponentRotation` _arrow) false false)
  ;[1 1 1] impulse 물리적인 힘 초기화
  (`PrimitiveComponent.SetAllPhysicsLinearVelocity` _ball (0.0 0.0 0.0) false)
  (`PrimitiveComponent.AddImpulse` _ball (* (`SceneComponent.GetForwardVector` _ball) 5000.0) "None" false))

(fn `UserConstructionScript`)